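; BP_Region_Parent is a parent Blueprint for a map region, apparently a French one, with a changeable colour.
; The construction script assigns the MeshRegion variable to the static mesh.
; ChangerCouleur creates a dynamic material instance on that mesh, sets its CouleurRegion parameter to the given colour and prints the value.
; Disconnected leftover nodes hold an unused DT_France_departement lookup and debug print.
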(event Collision|EventActorBeginOverlap
  (params (OtherActor :type Actor%20Object%20Reference)))

(event EventTick
  (params (DeltaSeconds :type Float%20%28single-precision%29)))

(event EventChangerCouleur
  (params (Couleur :type Linear%20Color%20Structure))
  (bind _returnvalue (Rendering|Material|CreateDynamicMaterialInstance (Variables|Default|GetStaticMesh) 0 0 "None" :!class /Script/Engine.PrimitiveComponent))
  (Rendering|Material|SetVectorParameterValue _returnvalue "CouleurRegion" Couleur :!class /Script/Engine.MaterialInstanceDynamic)
  (Development|PrintString (Utilities|String|ToString(Integer) Couleur)))

(fn ConstructionScript
  (Components|StaticMesh|SetStaticMesh (Variables|Default|GetStaticMesh) (Variables|Default|GetMeshRegion)))